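; BP_GameDirector is a level director actor that stages a sandstorm and the Sandman's arrival.
; OnCrystalPickedUp switches the Ultra Dynamic Weather actor to a calm sand-dust preset as a storm buildup.
; When the first-person character overlaps RealStormCollision, the weather turns to a full sand-dust storm and, after a delay, SpawnSandman is called on the character.
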(event `PrepareStorm`
  (bind _outactors (`GameplayStatics.GetAllActorsOfClass` "/Game/UltraDynamicSky/Blueprints/Ultra_Dynamic_Weather.Ultra_Dynamic_Weather_C"))
  (set `/Game/UltraDynamicSky/Blueprints/Ultra_Dynamic_Weather.Weather` "/Game/UltraDynamicSky/Blueprints/Weather_Effects/Weather_Presets/Sand_Dust_Calm.Sand_Dust_Calm" (`|GetArrayItem` _outactors)))

(event `StartRealStorm`
  (bind _outactors (`GameplayStatics.GetAllActorsOfClass` "/Game/UltraDynamicSky/Blueprints/Ultra_Dynamic_Weather.Ultra_Dynamic_Weather_C"))
  (set `/Game/UltraDynamicSky/Blueprints/Ultra_Dynamic_Weather.Weather` "/Game/UltraDynamicSky/Blueprints/Weather_Effects/Weather_Presets/Sand_Dust_Storm.Sand_Dust_Storm" (`|GetArrayItem` _outactors)))

(event `OnCrystalPickedUp`
  (`self.PrepareStorm`))

(event `self.RealStormCollision.OnComponentBeginOverlap`
  (params (OverlappedComponent :type "PrimitiveComponent Object Reference") (OtherActor :type "Actor Object Reference") (OtherComp :type "PrimitiveComponent Object Reference") (OtherBodyIndex :type Integer) (bFromSweep :type Boolean) (SweepResult :type "HitResult Structure (by ref)"))
  (cast `/Game/FirstPerson/Blueprints/BP_FirstPersonCharacter` OtherActor)
  (`self.StartRealStorm`)
  (`KismetSystemLibrary.Delay` 10.0)
  (bind _returnvalue (`GameplayStatics.GetActorOfClass` "/Game/FirstPerson/Blueprints/BP_FirstPersonCharacter.BP_FirstPersonCharacter_C"))
  (`/Game/FirstPerson/Blueprints/BP_FirstPersonCharacter.SpawnSandman` _returnvalue))

(fn `UserConstructionScript`)