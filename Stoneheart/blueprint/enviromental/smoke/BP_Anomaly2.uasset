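; BP_Anomaly2 is an environmental smoke anomaly whose Niagara effect pulses in scale while the first-person character is inside its box trigger.
; Entering the box sets an active flag and plays the Pulse timeline, which drives the Niagara component's world scale.
; On finish, the timeline restarts after a short delay while the flag holds.
; Leaving the box clears the flag, so the current pulse completes before stopping.
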(event `self.Box.OnComponentBeginOverlap`
  (params (OverlappedComponent :type "PrimitiveComponent Object Reference") (OtherActor :type "Actor Object Reference") (OtherComp :type "PrimitiveComponent Object Reference") (OtherBodyIndex :type Integer) (bFromSweep :type Boolean) (SweepResult :type "HitResult Structure (by ref)"))
  (cast `/Game/FirstPerson/Blueprints/BP_FirstPersonCharacter` OtherActor)
  (set `self.IsActive` true)
  (bind (_direction _newtrack_0) (`Timeline|pulse` :!via `PlayFromStart` :!label _label)
    (:`Update`
      (`SceneComponent.SetWorldScale3D` (`self.NewNiagaraSystem1`) (`KismetMathLibrary.Conv_DoubleToVector` _newtrack_0)))
    (:`Finished`
      (`KismetSystemLibrary.Delay` 0.02)
      (if (`self.IsActive`)
        (goto _label :!via `PlayFromStart`)))))

(event `self.Box.OnComponentEndOverlap`
  (params (OverlappedComponent :type "PrimitiveComponent Object Reference") (OtherActor :type "Actor Object Reference") (OtherComp :type "PrimitiveComponent Object Reference") (OtherBodyIndex :type Integer))
  (cast `/Game/FirstPerson/Blueprints/BP_FirstPersonCharacter` OtherActor)
  (set `self.IsActive` false))

(event `CustomEvent`
  (params (OverlappedComponent :type "PrimitiveComponent Object Reference") (OtherActor :type "Actor Object Reference") (OtherComp :type "PrimitiveComponent Object Reference") (OtherBodyIndex :type Integer)))

(fn `UserConstructionScript`)