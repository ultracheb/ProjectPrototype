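; BP_Smoke is an environmental effect actor whose FountainSmoke particles are periodically pushed by wind.
; From BeginPlay it loops forever, alternating a long calm interval with a shorter gust.
; Wind is faked by overriding the effect's Gravity variable: the replaying Rotate timeline varies its sideways component over a constant forward push.
; Ending the gust stops the timeline and points gravity straight down.
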(event `self.ReceiveBeginPlay`
  (`KismetSystemLibrary.Delay` 40.0 :!label _label)
  (`self.StartWind`)
  (`KismetSystemLibrary.Delay` 15.0)
  (`self.EndWind`)
  (goto _label))

(event `StartWind`
  (`NiagaraComponent.SetVariableVec3` (`self.FountainSmoke`) "Gravity" (1000.0 0.0 -100.0))
  (bind (_direction _newtrack_0) (`Timeline|Rotate` :!via `PlayFromStart` :!label _label_2)
    (:`Update`
      (`NiagaraComponent.SetVariableVec3` (`self.FountainSmoke`) "Gravity" (`KismetMathLibrary.MakeVector` 500.0 (* _newtrack_0 4.0) -100.0)))
    (:`Finished`
      (`KismetSystemLibrary.Delay` 0.2)
      (goto _label_2 :!via `PlayFromStart`))))

(event `EndWind`
  (`NiagaraComponent.SetVariableVec3` (`self.FountainSmoke`) "Gravity" (0.0 0.0 -1000.0))
  (goto _label_2 :!via `Stop`))

(fn `UserConstructionScript`)